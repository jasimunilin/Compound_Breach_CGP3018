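; Canvas-drawn HUD for the Compound Breach escape game, showing objective, keycard and power status, a crosshair, interaction prompt and controls hint.
; DrawHUD casts player character 0 to BP_EscapePlayer each frame and reads its state directly, drawing with DrawRect and DrawText instead of UMG.
; When the player's Escaped flag is set, it overlays a centered completion panel with a replay hint.
; A disconnected duplicate of the drawing chain remains in the graph and never runs.
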(event `self.ReceiveDrawHUD`
  (params (SizeX :type Integer) (SizeY :type Integer))
  (bind _asbp_escape_player (cast `/Game/CompoundBreach/Blueprints/BP_EscapePlayer` (`GameplayStatics.GetPlayerCharacter` 0)))
  (`self.DrawRect` (struct :`R` 0.015 :`G` 0.025 :`B` 0.035 :`A` 0.88) 24.0 24.0 610.0 118.0)
  (`self.DrawRect` (struct :`R` 0.1 :`G` 0.85 :`B` 0.75 :`A` 1) 24.0 24.0 4.0 118.0)
  (`self.DrawText` "COMPOUND / BREACH" (struct :`R` 0.1 :`G` 0.85 :`B` 0.75 :`A` 1) 42.0 36.0 null 1.5)
  (`self.DrawText` (`/Game/CompoundBreach/Blueprints/BP_EscapePlayer.Objective` _asbp_escape_player) (struct :`R` 1 :`G` 1 :`B` 1 :`A` 1) 42.0 69.0 null 1.1)
  (`self.DrawText` (select `bool` (`/Game/CompoundBreach/Blueprints/BP_EscapePlayer.HasKeycard` _asbp_escape_player) :`false` "KEYCARD: MISSING" :`true` "KEYCARD: ACQUIRED") (struct :`R` 0.85 :`G` 0.8 :`B` 0.55 :`A` 1) 42.0 108.0 null)
  (`self.DrawText` (select `bool` (`/Game/CompoundBreach/Blueprints/BP_EscapePlayer.PowerOnline` _asbp_escape_player) :`false` "POWER: OFFLINE" :`true` "POWER: ONLINE") (struct :`R` 0.85 :`G` 0.8 :`B` 0.55 :`A` 1) 280.0 108.0 null)
  (`self.DrawText` "+" (struct :`R` 1 :`G` 1 :`B` 1 :`A` 0.8) (- (* SizeX 0.5) 4.0) (- (* SizeY 0.5) 8.0) null)
  (`self.DrawRect` (struct :`R` 0.015 :`G` 0.025 :`B` 0.035 :`A` 0.8) 24.0 (- SizeY 76.0) 610.0 52.0)
  (`self.DrawText` (`/Game/CompoundBreach/Blueprints/BP_EscapePlayer.Prompt` _asbp_escape_player) (struct :`R` 0.2 :`G` 1 :`B` 0.8 :`A` 1) 42.0 (- SizeY 69.0) null 1.2)
  (`self.DrawText` "WASD  Move     MOUSE  Look     SPACE  Jump     E  Interact     R  Restart" (struct :`R` 0.65 :`G` 0.72 :`B` 0.78 :`A` 1) 42.0 (- SizeY 43.0) null)
  (if (`/Game/CompoundBreach/Blueprints/BP_EscapePlayer.Escaped` _asbp_escape_player)
    (`self.DrawRect` (struct :`R` 0.01 :`G` 0.03 :`B` 0.04 :`A` 0.92) (- (* SizeX 0.5) 260.0) (- (* SizeY 0.5) 80.0) 520.0 160.0)
    (`self.DrawText` "ESCAPE COMPLETE" (struct :`R` 0.1 :`G` 1 :`B` 0.75 :`A` 1) (- (* SizeX 0.5) 175.0) (- (* SizeY 0.5) 35.0) null 2.4)
    (`self.DrawText` "You restored power, secured access, and breached the compound." (struct :`R` 1 :`G` 1 :`B` 1 :`A` 1) (- (* SizeX 0.5) 220.0) (+ (* SizeY 0.5) 14.0) null)
    (`self.DrawText` "Press R to replay" (struct :`R` 1 :`G` 1 :`B` 1 :`A` 1) (- (* SizeX 0.5) 65.0) (+ (* SizeY 0.5) 42.0) null)))

(fn `UserConstructionScript`)